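; Gameplay ability that makes the player's Worker character dash in the move input direction, or along actor forward when there is almost no input.
; It snaps the avatar to face that direction, starts the dash montage and immediately applies a short root motion constant force with clamped exit velocity.
; The ability ends when the force finishes, leaving the montage playing, or immediately if the Pawn or SoulPlayerController cast fails.
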(event `self.K2_ActivateAbility`
  (bind _aspawn (cast `Pawn` (`self.GetAvatarActorFromActorInfo`))
    (:`then`
      (bind _assoul_player_controller (cast `SoulPlayerController` (`Pawn.GetController` _aspawn))
        (:`then`
          (bind _returnvalue (`SoulPlayerController.GetMoveInputDirection` _assoul_player_controller))
          (set `self.DashDirection` (`KismetMathLibrary.SelectVector` (`Actor.GetActorForwardVector` (`self.GetAvatarActorFromActorInfo`)) _returnvalue (< (`KismetMathLibrary.VSize` _returnvalue) 0.1)))
          (`Actor.K2_SetActorRotation` (`self.GetAvatarActorFromActorInfo`) (`KismetMathLibrary.Conv_VectorToRotator` (`self.DashDirection`)) false)
          (`AbilityTask_PlayMontageAndWait.CreatePlayMontageAndWaitProxy` "None" "/Game/Worker/Anim/WorkerDashMontage.WorkerDashMontage" 1.0 "None" false
            (:`then`
              (`AbilityTask_ApplyRootMotionConstantForce.ApplyRootMotionConstantForce` "None" (`self.DashDirection`) 1800.0 0.25 false null "ClampVelocity" (0.0 0.0 0.0) 200.0 true
                (:`OnFinish`
                  (`self.K2_EndAbility`))))))
        (:`CastFailed`
          (`self.K2_EndAbility` :!label _label))))
    (:`CastFailed`
      (goto _label))))