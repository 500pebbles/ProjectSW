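; Game mode that holds the player in place until the procedural map is generated, then moves them to the map entrance.
; On BeginPlay it finds the PMGMapBuilder, disables character movement and binds to its generation-finished event.
; On success it teleports the player with a fixed offset to the first PlayerStart whose name contains "_EntranceMarker".
; Walking is restored either way, with failure also printing a message.
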(event `self.ReceiveBeginPlay`
  ; 맵이 생성되기 전까지 이동을 멈춤
  (bind _returnvalue (`GameplayStatics.GetActorOfClass` "/Script/ProcMapGen.PMGMapBuilder"))
  (`/Engine/EditorBlueprintResources/StandardMacros.IsValid` _returnvalue
    (:`Is Valid`
      (`CharacterMovementComponent.DisableMovement` (`Character.CharacterMovement` (`GameplayStatics.GetPlayerCharacter` 0)))
      (add `PMGMapBuilder.OnGenerationFinished` _returnvalue (delegate `OnMapReady`)))))

(event `OnMapReady`
  (params (Result :type "PMGResult Structure (by ref)") (SpawnErrors :type "Array of String (by ref)"))
  (bind _returnvalue (`GameplayStatics.GetPlayerCharacter` 0))
  ; 맵 생성 성공여부를 판단하고 성공시 플레이어를 맵의 시작 지점 마커로 이동시키기
  (if (`.bSuccess` (break `PMGResult` Result))
    (bind _outactors (`GameplayStatics.GetAllActorsOfClass` "/Script/Engine.PlayerStart"))
    (for _array_element _outactors
      (if (`KismetStringLibrary.Contains` (`KismetSystemLibrary.GetObjectName` _array_element) "_EntranceMarker")
        (`self.K2_TeleportTo` _returnvalue (+ (`self.K2_GetActorLocation` _array_element) (200.0 0.0 100.0)) (`self.K2_GetActorRotation` _array_element))
        (break)))
    (else
      (`KismetSystemLibrary.PrintString` "맵 생성 실패")))
  (`CharacterMovementComponent.SetMovementMode` (`Character.CharacterMovement` _returnvalue) "MOVE_Walking" 0))

(fn `UserConstructionScript`)