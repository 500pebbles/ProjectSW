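; BP_L_Room1x1_D is a 1x1 room Blueprint that hosts a shop.
; On BeginPlay it runs the parent logic, spawns a BP_ShopActor at its ShopSpawnPoint component with itself as owner, and attaches the shop there.
; On EndPlay it destroys the spawned shop if still valid, so the shop's lifetime follows the room's.
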(event `self.ReceiveBeginPlay`
  (`parent.ReceiveBeginPlay`)
  (bind _returnvalue (`|SpawnActorFromClass` "/Game/Blueprints/Shop/BP_ShopActor.BP_ShopActor_C" (`SceneComponent.K2_GetComponentToWorld` (`self.ShopSpawnPoint`)) "AlwaysSpawn" "MultiplyWithRoot" self null))
  (bind _output_get (set `self.SpawnedShop` _returnvalue))
  (`self.K2_AttachToComponent` _output_get (`self.ShopSpawnPoint`) "None" "KeepWorld" "KeepWorld" "KeepWorld" true))

(event `self.ReceiveEndPlay`
  (params (EndPlayReason :type "EEndPlayReason Enum" :default "Destroyed"))
  (bind _spawnedshop (`self.SpawnedShop`))
  (`parent.ReceiveEndPlay` EndPlayReason)
  (if (`KismetSystemLibrary.IsValid` _spawnedshop)
    (`self.K2_DestroyActor` _spawnedshop)))

(fn `UserConstructionScript`
  (`parent.UserConstructionScript`))