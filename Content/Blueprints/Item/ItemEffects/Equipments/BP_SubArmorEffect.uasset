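; Equipment item effect for sub armor that boosts the wearer's max health, defense and critical rate through the Gameplay Ability System.
; Activation builds a GE_SubArmor spec, fills its set-by-caller tags with the item's scaled effect values, applies it to the user and stores the active handle.
; Deactivation removes the effect by that handle and, on success, clears the handle and item reference.
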(event `self.ActivateItemEffect`
  (params (User :type "Actor Object Reference") (Item :type "ItemData Object Reference"))
  (bind _returnvalue (`AbilitySystemBlueprintLibrary.GetAbilitySystemComponent` User))
  (bind _output_get (set `self.Item` Item))
  (bind _returnvalue_2 (`AbilitySystemBlueprintLibrary.AssignTagSetByCallerMagnitude` (`AbilitySystemComponent.MakeOutgoingSpec` :`self` _returnvalue :`GameplayEffectClass` "/Game/Blueprints/GAS/GE/Item/Equipment/GE_SubArmor.GE_SubArmor_C") (struct :`TagName` "SoulTags.Attributes.MaxHealth") (`ItemData.GetScaledEffectValue` _output_get 0)))
  (bind _returnvalue_3 (`AbilitySystemBlueprintLibrary.AssignTagSetByCallerMagnitude` _returnvalue_2 (struct :`TagName` "SoulTags.Attributes.Defense") (`ItemData.GetScaledEffectValue` _output_get 1)))
  (bind _returnvalue_4 (`AbilitySystemBlueprintLibrary.AssignTagSetByCallerMagnitude` _returnvalue_3 (struct :`TagName` "SoulTags.Attributes.CriticalRate") (`ItemData.GetScaledEffectValue` _output_get 2)))
  (bind _returnvalue_5 (`AbilitySystemComponent.BP_ApplyGameplayEffectSpecToTarget` _returnvalue _returnvalue_4 _returnvalue))
  (set `self.GameplayEffectHandle` _returnvalue_5))

(event `self.DeactivateItemEffect`
  (params (User :type "Actor Object Reference") (Item :type "ItemData Object Reference"))
  (bind _returnvalue (`AbilitySystemComponent.RemoveActiveGameplayEffect` (`AbilitySystemBlueprintLibrary.GetAbilitySystemComponent` User) (`self.GameplayEffectHandle`) -1))
  (if _returnvalue
    (`AbilitySystemBlueprintLibrary.IsActiveGameplayEffectHandleValid` (`self.GameplayEffectHandle`))
    (set `self.GameplayEffectHandle` (struct))
    (set `self.Item` null)))