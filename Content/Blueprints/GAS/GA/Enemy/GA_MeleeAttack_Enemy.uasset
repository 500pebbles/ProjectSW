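; GA_MeleeAttack_Enemy is a gameplay ability for an enemy melee attack, so far without damage logic.
; It faces the avatar toward its combat target through SoulCombatInterface (labeled Motion Warp), then plays the attack montage.
; A melee montage gameplay event draws a debug sphere at the combat socket and ends the ability.
; Montage interruption, cancellation or a failed interface cast also ends it.
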(event `self.K2_ActivateAbility`
  (bind _returnvalue (`self.GetAvatarActorFromActorInfo`))
  ; Motion Warp
  (bind _returnvalue_2 (message `SoulCombatInterface.GetCombatTarget` _returnvalue))
  (bind _assoul_combat_interface (cast `SoulCombatInterface` _returnvalue)
    (:`then`
      (`SoulCombatInterface.FaceToTarget` _assoul_combat_interface (`Actor.K2_GetActorLocation` _returnvalue_2))
      ; PlayMontage and WaitGameplayEvent
      (`AbilityTask_PlayMontageAndWait.CreatePlayMontageAndWaitProxy` "None" "/Game/Assets/Dummy/UE5_Mannequin/Anims/Unarmed/Attack/AM_Enemy_Attack_01.AM_Enemy_Attack_01"
        (:`then`
          (`AbilityTask_WaitGameplayEvent.WaitGameplayEvent` (struct :`TagName` "SoulTags.Events.Montages.Attacks.Melee") null
            (:`EventReceived`
              (bind _returnvalue_3 (message `SoulCombatInterface.GetCombatSocketLocation` (`self.GetAvatarActorFromActorInfo`)))
              (`KismetSystemLibrary.DrawDebugSphere` _returnvalue_3 45.0 12 (struct :`R` 0.359937 :`G` 1.0 :`B` 0.179046 :`A` 1.0) 0.5)
              (`self.K2_EndAbility`))))
        (:`OnInterrupted`
          (`self.K2_EndAbility` :!label _label))
        (:`OnCancelled`
          (goto _label))))
    (:`CastFailed`
      (`self.K2_EndAbility`))))