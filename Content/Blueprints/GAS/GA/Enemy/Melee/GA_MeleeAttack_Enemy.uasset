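; Gameplay Ability for enemy melee attacks that turns the avatar toward its combat target and plays a random tagged attack montage.
; The montage's gameplay event triggers a radius search at the combat socket, damages every non-allied actor found with a debug sphere drawn on each, then ends the ability.
; The ability also ends if the montage completes, is interrupted or cancelled, or the avatar lacks the combat interface.
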(event `self.K2_ActivateAbility`
  (bind _returnvalue (`self.GetAvatarActorFromActorInfo`))
  (bind _returnvalue_2 (`self.GetAvatarActorFromActorInfo`))
  ; Motion Warp
  (bind _returnvalue_3 (message `SoulCombatInterface.GetCombatTarget` _returnvalue))
  (bind _assoul_combat_interface (cast `SoulCombatInterface` _returnvalue)
    (:`then`
      (`SoulCombatInterface.FaceToTarget` _assoul_combat_interface (`Actor.K2_GetActorLocation` _returnvalue_3))
      ; PlayMontage and WaitGameplayEvent
      (bind _returnvalue_4 (message `SoulCombatInterface.GetAttackMontages` (`self.GetAvatarActorFromActorInfo`)))
      (bind _output_get (set `self.TaggedMontage` (`self.GetRandomTaggedMontage` _returnvalue_4)))
      (bind (_montage _montagetag) (break `TaggedMontage` _output_get))
      (`AbilityTask_PlayMontageAndWait.CreatePlayMontageAndWaitProxy` "None" _montage 1.0 "None" false
        (:`then`
          (`AbilityTask_WaitGameplayEvent.WaitGameplayEvent` _montagetag null
            (:`EventReceived`
              ; Get All Targets in Combat Location
              (bind _returnvalue_5 (message `SoulCombatInterface.GetCombatSocketLocation` (`self.GetAvatarActorFromActorInfo`)))
              (bind _outoverlappingactors (`SoulAbilitySystemLibrary.GetActorsWithinRadius` _returnvalue_2 (`|MakeArray` _returnvalue_2) 50.0 _returnvalue_5))
              ; Apply Damage
              (for _array_element _outoverlappingactors
                (if (not (`SoulAbilitySystemLibrary.AreActorsAllies` _array_element (`self.GetAvatarActorFromActorInfo`)))
                  (`self.ApplyDamage` _array_element)
                  (`KismetSystemLibrary.DrawDebugSphere` (`Actor.K2_GetActorLocation` _array_element) 45.0 12 (struct :`R` 0.359937 :`G` 1.0 :`B` 0.179046 :`A` 1.0) 0.5)))
              (`self.K2_EndAbility`))))
        (:`OnCompleted`
          (`self.K2_EndAbility` :!label _label))
        (:`OnInterrupted`
          (goto _label))
        (:`OnCancelled`
          (goto _label))))
    (:`CastFailed`
      (`self.K2_EndAbility`))))