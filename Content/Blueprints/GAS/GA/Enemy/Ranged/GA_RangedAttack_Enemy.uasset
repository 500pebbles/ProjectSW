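; Gameplay ability for an enemy ranged attack that turns the avatar toward its combat target and fires a projectile during an attack animation.
; It queries the avatar through messages for its target and attack montages, then plays a randomly chosen tagged montage.
; The montage's gameplay event tag triggers the projectile spawn.
; The ability ends when the montage completes, is interrupted or is cancelled.
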(event `self.K2_ActivateAbility`
  (bind _returnvalue (message `SoulCombatInterface.GetCombatTarget` (`self.GetAvatarActorFromActorInfo`)))
  (message `SoulCombatInterface.FaceToTarget` (`self.GetAvatarActorFromActorInfo`) (`Actor.K2_GetActorLocation` _returnvalue))
  (bind _returnvalue_2 (message `SoulCombatInterface.GetAttackMontages` (`self.GetAvatarActorFromActorInfo`)))
  (bind _output_get (set `self.TaggedMontage` (`self.GetRandomTaggedMontage` _returnvalue_2)))
  (bind (_montage _montagetag) (break `TaggedMontage` _output_get))
  (`AbilityTask_PlayMontageAndWait.CreatePlayMontageAndWaitProxy` "None" _montage 1.0 "None" false
    (:`then`
      (`AbilityTask_WaitGameplayEvent.WaitGameplayEvent` _montagetag null
        (:`EventReceived`
          (message `SoulCombatInterface.GetCombatSocketLocation` (`self.GetAvatarActorFromActorInfo`))
          (bind _returnvalue_3 (message `SoulCombatInterface.GetCombatTarget` (`self.GetAvatarActorFromActorInfo`)))
          (`self.SpawnProjectile`))))
    (:`OnCompleted`
      (`self.K2_EndAbility` :!label _label))
    (:`OnInterrupted`
      (goto _label))
    (:`OnCancelled`
      (goto _label))))