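; Player melee attack Gameplay Ability that plays an attack montage as a multi-section combo and ends with it.
; Montage gameplay events drive hit detection, damaging each target once per trace with a per-step multiplier.
; Combo Open, Branch and Close events define the input window: early presses buffer until Branch, later ones chain immediately.
; Each chained hit turns the avatar toward the attack direction consumed from SoulPlayerController before jumping sections.
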(event `GoNextHit`
  ; 다음 공격으로 전환
  (if (< (`self.ComboIndex`) (`KismetArrayLibrary.Array_LastIndex` (`self.ComboSections`)))
    (`/Engine/EditorBlueprintResources/StandardMacros.IncrementInt` (`self.ComboIndex`)
      (:`  `
        (set `self.bWindowOpen` false)
        (set `self.bBranchPassed` false)
        (set `self.bInputBuffered` false)
        (`self.RotateToAttackInput`)
        (`self.MontageJumpToSection` (`|GetArrayItem` (`self.ComboSections`) (`self.ComboIndex`)))))))

(event `self.K2_ActivateAbility`
  ; 공격 진입용 초기화 시점
  (set `self.ComboIndex` 0)
  (set `self.bWindowOpen` false)
  (set `self.bBranchPassed` false)
  (set `self.bInputBuffered` false)
  (`self.ClearAttackInput`)
  (`BlueprintSetLibrary.Set_Clear` (`self.HitActors`))
  ; 공격 시동과 데미지 판정
  (`AbilityTask_PlayMontageAndWait.CreatePlayMontageAndWaitProxy` "None" "/Game/Blueprints/Character/Player/Chii/WorkerAttack_Montage.WorkerAttack_Montage" 1.0 "Attack1"
    (:`then`
      (`AbilityTask_WaitGameplayEvent.WaitGameplayEvent` (struct :`TagName` "SoulTags.Events.Melee.TraceBegin") null
        (:`then`
          (bind (_asynctaskproxy _payload) (`AbilityTask_WaitGameplayEvent.WaitGameplayEvent` (struct :`TagName` "SoulTags.Events.Melee.Hit") null)
            (:`then`
              ; 콤보 입력 처리
              (`AbilityTask_WaitGameplayEvent.WaitGameplayEvent` (struct :`TagName` "SoulTags.Events.Combo.Open") null
                (:`then`
                  (`AbilityTask_WaitGameplayEvent.WaitGameplayEvent` (struct :`TagName` "SoulTags.Events.Combo.Close") null
                    (:`then`
                      (`AbilityTask_WaitGameplayEvent.WaitGameplayEvent` (struct :`TagName` "SoulTags.Events.Combo.Branch") null
                        (:`then`
                          (`AbilityTask_WaitInputPress.WaitInputPress` false :!label _label
                            (:`OnPress`
                              (`self.HandleComboInput`)
                              (goto _label))))
                        (:`EventReceived`
                          (if (`self.bInputBuffered`)
                            (`self.GoNextHit` :!label _label_2)
                            (else
                              (set `self.bBranchPassed` true))))))
                    (:`EventReceived`
                      (set `self.bWindowOpen` false))))
                (:`EventReceived`
                  (set `self.bWindowOpen` true)
                  (set `self.bBranchPassed` false)
                  (set `self.bInputBuffered` false))))
            (:`EventReceived`
              (bind (_eventtag _instigator _target) (break `GameplayEventData` _payload))
              (if (not (`BlueprintSetLibrary.Set_Contains` (`self.HitActors`) _target))
                (`BlueprintSetLibrary.Set_Add` (`self.HitActors`) _target)
                (`self.ApplyMeleeDamage` _target (`|GetArrayItem` (`self.DamageMultipliers`) (`self.ComboIndex`)))))))
        (:`EventReceived`
          (`BlueprintSetLibrary.Set_Clear` (`self.HitActors`)))))
    (:`OnCompleted`
      (`self.K2_EndAbility` :!label _label_3))
    (:`OnBlendOut`
      (goto _label_3))
    (:`OnInterrupted`
      (goto _label_3))
    (:`OnCancelled`
      (goto _label_3))))

(event `HandleComboInput`
  ; 콤보 입력 처리
  (if (`self.bWindowOpen`)
    (if (`self.bBranchPassed`)
      (goto _label_2)
      (else
        (set `self.bInputBuffered` true)))))

(fn `ClearAttackInput`
  (bind _soulpc (`self.GetSoulPC`))
  (`/Engine/EditorBlueprintResources/StandardMacros.IsValid` _soulpc
    (:`Is Valid`
      (`SoulPlayerController.ConsumeAttackInputDirection` _soulpc))))

(fn `GetSoulPC`
  (returns (SoulPC :type "SoulPlayerController Object Reference"))
  (locals (NewLocalVar :type "SoulPlayerController Object Reference"))
  (bind `_as폰` (cast `Pawn` (`self.GetAvatarActorFromActorInfo`)))
  (bind _assoul_player_controller (cast `SoulPlayerController` (`Pawn.GetController` `_as폰`)))
  (return _assoul_player_controller))

(fn `RotateToAttackInput`
  (bind _soulpc (`self.GetSoulPC`))
  (`/Engine/EditorBlueprintResources/StandardMacros.IsValid` _soulpc
    (:`Is Valid`
      (bind _returnvalue (`SoulPlayerController.ConsumeAttackInputDirection` _soulpc))
      (if (> (`KismetMathLibrary.VSize` _returnvalue) 0.1)
        (`Actor.K2_SetActorRotation` (`self.GetAvatarActorFromActorInfo`) (`KismetMathLibrary.Conv_VectorToRotator` _returnvalue) false)))))